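; AI character that fires projectiles, takes damage and respawns at random spawn points.
; Start and stop events control a looping timer that spawns AiProj at Arrow1 every RateOfFire seconds.
; Damage reduces and prints Health; at zero the character is moved far below the origin, then after a delay regains health and teleports to a SpawnerPoint gathered at BeginPlay.
; A HealthBonus event sets Health to a supplied maximum.
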(event Custom|AiSHoot
  ;[1 1 1] Projectile
  ;;[1 1 1] spawn_projectile
  (Game|SpawnActorfromClass "/Game/AI/aiProj.aiProj_C" (Transformation|GetWorldTransform (Variables|Default|GetArrow1)) "Undefined" "MultiplyWithRoot" self 0))

(event Custom|startshooting
  ;[1 1 1] Projectile
  (Utilities|Time|SetTimerbyFunctionName 0 "AiSHoot" (Variables|Default|GetRateOfFire) true))

(event Custom|stop_shooting
  ;[1 1 1] Projectile
  (Utilities|Time|ClearTimerbyFunctionName 0 "AiSHoot"))

(event Custom|CheckHealth
  ;[1 1 1] Health and damage
  (if (<= (Variables|Default|GetHealth) 0.0)
    (Transformation|SetActorLocation "0.000000,0.000000,-5000.000000" false false)
    (CallFunction|Respawn)))

(event Custom|HealthBonus
  (params (maxHealth :type Float%20%28double-precision%29))
  ;[1 1 1] Health and damage
  (bind _output_get (Variables|Default|SetmaxHealth maxHealth))
  (Variables|Default|SetHealth _output_get))

(event Custom|Respawn
  (bind _spawnpoints (Variables|Default|GetSpawnPoints))
  ;[1 1 1] Resapwn
  (Utilities|FlowControl|Delay 2.0)
  (Variables|Default|SetHealth 1e+02)
  (Transformation|SetActorLocation (Transformation|GetActorLocation (Utilities|Array|Get(acopy) _spawnpoints (Math|Random|RandomIntegerinRange 0 (- (Utilities|Array|Length _spawnpoints) 1)))) false true))

(event EventBeginPlay
  ;[1 1 1] Resapwn
  (bind _outactors (Actor|GetAllActorsOfClass "/Game/spawner/spawnerPoint.spawnerPoint_C"))
  (Variables|Default|SetSpawnPoints _outactors))

(event Game|Damage|EventAnyDamage
  (params (Damage :type Float%20%28single-precision%29) (DamageType :type Damage%20Type%20Object%20Reference) (InstigatedBy :type Controller%20Object%20Reference) (DamageCauser :type Actor%20Object%20Reference))
  ;[1 1 1] Health and damage
  (Variables|Default|SetDamage%20Causer DamageCauser)
  (Variables|Default|SetHealth (- (Variables|Default|GetHealth) Damage))
  (CallFunction|CheckHealth)
  (Development|PrintString (Utilities|String|ToString(Float) (Variables|Default|GetHealth)) true true "(R=0.500000,G=0.004591,B=0.000000,A=1.000000)"))

(fn ConstructionScript)