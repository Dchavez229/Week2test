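; Player character Blueprint that handles movement, look, jumping and firing.
; Movement axes add input along forward and right vectors derived from control rotation, with forward using yaw only, while look axes drive controller pitch and yaw.
; The jump action starts and stops jumping, and pressing fire spawns a PlayerProj_BP projectile at the Arrow1 component's world transform.
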(event EventBeginPlay)

(event Input|ActionEvents|InputActionjump
  (params (Key :type Key%20Structure :default "None"))
  ;[0.3783 0.9101 1] jumping
  (:Pressed
    (Character|Jump))
  (:Released
    (Character|StopJumping)))

(event Input|ActionEvents|InputActionfire
  (params (Key :type Key%20Structure :default "None"))
  (:Pressed
    (Game|SpawnActorfromClass "/Game/player/playerProj_BP.playerProj_BP_C" (Transformation|GetWorldTransform (Variables|Default|GetArrow1)) "Undefined" "MultiplyWithRoot" 0 0)))

(event Input|AxisEvents|InputAxismoveForward
  (params (AxisValue :type Float%20%28single-precision%29))
  ;[0.7865 0.252 1] movement
  (Pawn|Input|AddMovementInput (Math|Vector|GetForwardVector (Math|Rotator|MakeRotator 0.0 0.0 (.yaw (Pawn|GetControlRotation :!class /Script/Engine.Pawn)))) AxisValue false))

(event Input|AxisEvents|InputAxisMoveRight
  (params (AxisValue :type Float%20%28single-precision%29))
  (bind _returnvalue (Pawn|GetControlRotation :!class /Script/Engine.Pawn))
  ;[0.7865 0.252 1] movement
  (Pawn|Input|AddMovementInput (Math|Vector|GetRightVector (Math|Rotator|MakeRotator (.roll _returnvalue) 0.0 (.yaw _returnvalue))) AxisValue false))

(event Input|AxisEvents|InputAxisLookUp
  (params (AxisValue :type Float%20%28single-precision%29))
  ;[1 0.1354 0.1354] look
  (Pawn|Input|AddControllerPitchInput AxisValue))

(event Input|AxisEvents|InputAxisTurn
  (params (AxisValue :type Float%20%28single-precision%29))
  ;[1 0.1354 0.1354] look
  (Pawn|Input|AddControllerYawInput AxisValue))

(fn ConstructionScript)